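; BP_Weapon is a pickup melee weapon that can be equipped and deals damage through swept hit detection.
; On pickup, it sends itself to the interactor's equip interface and disables its trigger collision.
; While Istracing is set, Tick runs a debug-drawn box trace between TraceStart and TraceEnd, ignoring the attach parent.
; HasHit latches on the first actor with AC_Attributes, which receives a fixed-damage hit message.
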(event `self.ReceiveTick`
  (params (DeltaSeconds :type "Float (single-precision)"))
  (if (`self.istracing`)
    (`self.PerformWeapontrace`)))

(event `self.PickUp`
  (params (InteractingActor :type "Actor Object Reference"))
  (bind _trigger (`self.trigger`))
  (if (`KismetSystemLibrary.DoesImplementInterface` InteractingActor "/Game/Blueprints/Characters/BPI_EquipInterface.BPI_EquipInterface_C")
    (`KismetSystemLibrary.PrintString` "equipped weapon")
    (message `/Game/Blueprints/Characters/BPI_EquipInterface.Equip` InteractingActor self)
    (`PrimitiveComponent.SetCollisionEnabled` _trigger "NoCollision")
    (set `PrimitiveComponent.bGenerateOverlapEvents` false _trigger)))

(fn `PerformWeapontrace`
  (bind _tracestart (`self.TraceStart`))
  (if (not (`self.HasHit`))
    (bind (_outhit _returnvalue) (`KismetSystemLibrary.BoxTraceSingle` (`SceneComponent.K2_GetComponentLocation` _tracestart) (`SceneComponent.K2_GetComponentLocation` (`self.TraceEnd`)) (5.0 5.0 30.0) (`SceneComponent.K2_GetComponentRotation` _tracestart) "TraceTypeQuery1" false (`|MakeArray` (`self.GetAttachParentActor`)) "ForDuration"))
    (if _returnvalue
      (`KismetSystemLibrary.PrintString` "hit")
      (bind (_bblockinghit _binitialoverlap _time _distance _location _impactpoint _normal _impactnormal _physmat _hitactor) (`GameplayStatics.BreakHitResult` _outhit))
      (if (`KismetSystemLibrary.IsValid` (`self.GetComponentByClass` _hitactor "/Game/Blueprints/AC_Attributes.AC_Attributes_C"))
        (set `self.HasHit` true)
        (message `/Game/Blueprints/BPI_Combat.GetHit` _hitactor 50.0)))))

(fn `UserConstructionScript`
  (`parent.UserConstructionScript`))