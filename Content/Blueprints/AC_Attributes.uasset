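; Attribute component that tracks health and stamina and broadcasts their changes through event dispatchers.
; TakeDamage subtracts health, firing OnDeath at zero or below and OnHealthChanged otherwise, while ResetHealth restores maximum health without broadcasting.
; Stamina has separate check and pay functions, and Tick regenerates it at the StaminaCost regen rate while below maximum, broadcasting each update without clamping the result.
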(event `self.ReceiveBeginPlay`
  (set `self.Health` (`self.MaxHealth`))
  (`self.OnStaminaChanged` (`self.Stamina`) (`self.MaxStamina`) :!label _label))

(event `self.ReceiveTick`
  (params (DeltaSeconds :type "Float (single-precision)"))
  (bind _stamina (`self.Stamina`))
  (bind _staminacost_staminaregenrate (break `/Game/Blueprints/ST_StaminaCost` (`self.StaminaCost`)))
  (if (< _stamina (`self.MaxStamina`))
    (set `self.Stamina` (+ (* (`GameplayStatics.GetWorldDeltaSeconds`) _staminacost_staminaregenrate) _stamina))
    (goto _label)))

(fn `CanPayStaminaCost`
  (params (Cost :type "Float (double-precision)"))
  (returns (Can :type Boolean))
  (return (>= (`self.Stamina`) Cost)))

(fn `PayStamina`
  (params (Cost :type "Float (double-precision)"))
  (bind _stamina (`self.Stamina`))
  (set `self.Stamina` (- _stamina Cost))
  (`self.OnStaminaChanged` _stamina (`self.MaxStamina`)))

(fn `ResetHealth`
  (set `self.Health` (`self.MaxHealth`)))

(fn `TakeDamage`
  (params (Damage :type "Float (double-precision)"))
  (bind _health (`self.Health`))
  (set `self.Health` (- _health Damage))
  (if (<= _health 0.0)
    (`self.OnDeath`)
    (else
      (`self.OnHealthChanged` (`self.Health`) (`self.MaxHealth`)))))