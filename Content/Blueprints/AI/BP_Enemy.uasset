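; BP_Enemy is a melee enemy that picks up overlapping items on BeginPlay and attaches equipped weapons to its WeaponSocket.
; Attack plays a montage gated by PawnState, while separate events toggle the weapon's hitbox and tracing.
; GetHit routes damage to AC_Attributes, which drives the death montage; a separate OnDeath event destroys the actor.
; A line-trace attack on the player is left unconnected and never runs.
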(event `/Game/Blueprints/BPI_Combat.EnableWeaponHitbox`
  (bind _weapon (`self.weapon`))
  (bind _hitbox (`/Game/Blueprints/BP_Weapon.hitbox` _weapon))
  (`PrimitiveComponent.SetCollisionEnabled` _hitbox "QueryOnly")
  (set `PrimitiveComponent.bGenerateOverlapEvents` true _hitbox)
  (set `/Game/Blueprints/BP_Weapon.istracing` true _weapon)
  (set `/Game/Blueprints/BP_Weapon.HasHit` false _weapon :!label _label))

(event `/Game/Blueprints/BPI_Combat.DisableWeaponHitbox`
  (bind _weapon (`self.weapon`))
  (bind _hitbox (`/Game/Blueprints/BP_Weapon.hitbox` _weapon))
  (`PrimitiveComponent.SetCollisionEnabled` _hitbox "NoCollision")
  (set `PrimitiveComponent.bGenerateOverlapEvents` false _hitbox)
  (set `/Game/Blueprints/BP_Weapon.istracing` false _weapon)
  (goto _label))

(event `/Game/Blueprints/Characters/BPI_EquipInterface.Equip`
  (params (Item :type "/Game/Blueprints/BP_Weapon Object Reference"))
  (`self.K2_AttachToComponent` Item (`self.Mesh`) "WeaponSocket" "SnapToTarget" "SnapToTarget" "KeepWorld" true)
  (set `self.weapon` Item))

(event `self.ReceiveBeginPlay`
  (set `self.PawnState` "NewEnumerator0")
  (for _array_element (`self.GetOverlappingActors` "/Game/Blueprints/BP_Item.BP_Item_C")
    (if (`KismetSystemLibrary.DoesImplementInterface` _array_element "/Game/Blueprints/BPI_Interaction.BPI_Interaction_C")
      (message `/Game/Blueprints/BPI_Interaction.PickUp` _array_element self))))

(event `self.ReceiveTick`
  (params (DeltaSeconds :type "Float (single-precision)")))

(event `self.GetHit`
  (params (Damage :type "Float (double-precision)"))
  (bind _ac_attributes (`self.AC_Attributes`))
  (`/Game/Blueprints/AC_Attributes.TakeDamage` _ac_attributes Damage)
  (if (not (<= (`/Game/Blueprints/AC_Attributes.Health` _ac_attributes) 0.0))
    (`self.PlayAnimMontage` "/Game/Assets/Animations/AM_Getting_Hit_Montage.AM_Getting_Hit_Montage")))

(event `self.AC_Attributes.OnDeath`
  (`self.PlayAnimMontage` "/Game/Assets/Animations/AM_Standing_React_Death_Backward_Montage.AM_Standing_React_Death_Backward_Montage"))

(event `/Game/Blueprints/BPI_Combat.OnDeath`
  (`self.K2_DestroyActor`))

(fn `Attack`
  (if (`|EnumEquality` (`self.PawnState`) "NewEnumerator0")
    (set `self.PawnState` "NewEnumerator2")
    (`self.PlayAnimMontage` "/Game/Assets/Animations/AM_Standing_Melee_Attack_Downward_Montage.AM_Standing_Melee_Attack_Downward_Montage")))

(fn `UserConstructionScript`)