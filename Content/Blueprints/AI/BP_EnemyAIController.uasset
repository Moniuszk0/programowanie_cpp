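; AI controller for enemies that runs the BT_Enemy behavior tree on the BB_Enemy blackboard when it possesses a pawn.
; Perception updates write the target actor, last known player location and visibility flag, clearing the target when sensing fails.
; Tick sets an in-attack-range flag from the pawn's distance to the current target, updating it only while a target exists.
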(event `self.ReceiveTick`
  (params (DeltaSeconds :type "Float (single-precision)"))
  (bind _blackboard_component (`self.Blackboard Component`))
  (bind (_asactor _bsuccess) (cast `Actor` (`BlackboardComponent.GetValueAsObject` _blackboard_component "TargetActor") :!pure true))
  (if _bsuccess
    (`BlackboardComponent.SetValueAsBool` _blackboard_component "InAttackRange" (<= (`KismetMathLibrary.Vector_Distance` (`self.K2_GetActorLocation` _asactor) (`self.K2_GetActorLocation` (`self.K2_GetPawn`))) 200.0))))

(event `self.ReceivePossess`
  (params (PossessedPawn :type "Pawn Object Reference"))
  (bind _blackboardcomponent (`self.UseBlackboard` "/Game/Blueprints/AI/BB_Enemy.BB_Enemy"))
  (set `self.Blackboard Component` _blackboardcomponent)
  (`self.RunBehaviorTree` "/Game/Blueprints/AI/BT_Enemy.BT_Enemy"))

(event `self.AIPerception.OnTargetPerceptionUpdated`
  (params (Actor :type "Actor Object Reference") (Stimulus :type "AIStimulus Structure"))
  (bind _returnvalue (`self.K2_GetActorLocation` Actor))
  (bind _blackboard_component (`self.Blackboard Component`))
  (if (`.bSuccessfullySensed` (break `AIStimulus` Stimulus))
    (`BlackboardComponent.SetValueAsObject` _blackboard_component "TargetActor" Actor)
    (`BlackboardComponent.SetValueAsVector` _blackboard_component "LastKnownPlayerLocation" _returnvalue)
    (`BlackboardComponent.SetValueAsBool` _blackboard_component "CanSeePlayer" true)
    (else
      (`BlackboardComponent.ClearValue` _blackboard_component "TargetActor")
      (`BlackboardComponent.SetValueAsVector` _blackboard_component "LastKnownPlayerLocation" _returnvalue)
      (`BlackboardComponent.SetValueAsBool` _blackboard_component "CanSeePlayer" false))))

(fn `UserConstructionScript`)