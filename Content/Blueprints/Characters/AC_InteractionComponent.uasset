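; Actor component that line traces ahead of its owner, apparently as an unfinished base for interaction.
; Every Tick it traces on the Visibility channel from the owner's location along its forward vector for TraceDistance, with debug drawing on.
; The hit result drives nothing, as the logic to clear CurrentInteractable on an invalid hit is disconnected.
; A node setting TraceDistance is also unconnected.
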(event `self.ReceiveTick`
  (params (DeltaSeconds :type "Float (single-precision)"))
  (bind _returnvalue (`self.GetOwner`))
  (bind _returnvalue_2 (`Actor.K2_GetActorLocation` _returnvalue))
  (bind _outhit (`KismetSystemLibrary.LineTraceSingle` :`Start` _returnvalue_2 :`End` (+ _returnvalue_2 (* (`Actor.GetActorForwardVector` _returnvalue) (`self.TraceDistance`))) :`TraceChannel` "TraceTypeQuery1" :`DrawDebugType` "ForDuration")))